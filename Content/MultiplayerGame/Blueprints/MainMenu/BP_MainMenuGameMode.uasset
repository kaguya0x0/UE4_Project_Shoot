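; Game mode for the main menu of a multiplayer game, handling menu screens and session hosting and joining.
; Separate events create and show the main, host, server and option menu widgets.
; Hosting saves server settings to the game instance, creates a session and opens the Lobby as a listen server.
; The game instance shows loading screens and failure messages, and a failed join returns to the main menu.
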(event Custom|ShowServerMenu
  (bind _returnvalue (UserInterface|CreateWidget "/Game/MultiplayerGame/Blueprints/Widget/MainMenu/WBP_ServerMenu.WBP_ServerMenu_C" (Game|GetPlayerController 0)))
  (UserInterface|Viewport|AddtoViewport _returnvalue 0))

(event Custom|ShowOptionMenu
  (bind _returnvalue (UserInterface|CreateWidget "/Game/MultiplayerGame/Blueprints/Widget/MainMenu/WBP_OptionMenu.WBP_OptionMenu_C" (Game|GetPlayerController 0)))
  (UserInterface|Viewport|AddtoViewport _returnvalue 0))

(event Custom|HostGame
  (params (ServerName :type Text) (MaxPlayer :type Integer) (UseLAN :type Boolean))
  (bind _returnvalue (Game|GetGameInstance))
  (bind _asbp_game_instance (Utilities|Casting|CastToBP_GameInstance _returnvalue))
  (Variables|/Game/MultiplayerGame/Blueprints/General/BP_GameInstance.BP_GameInstance_C|SetServerName _asbp_game_instance ServerName)
  (Variables|/Game/MultiplayerGame/Blueprints/General/BP_GameInstance.BP_GameInstance_C|SetMaxPlayer _asbp_game_instance MaxPlayer)
  (CallFunction|ShowLoadingScreen)
  (|Session (Game|GetPlayerController 0) MaxPlayer UseLAN
    (:OnSuccess
      (Game|OpenLevel(byName) "Lobby" true "listen"))
    (:OnFailure
      (Default|ShowMessageWindow _asbp_game_instance "Failed to Create Session. Please Try Again."))))

(event Custom|JoinGame
  (params (Session :type Blueprint%20Session%20Result%20Structure))
  (CallFunction|ShowLoadingScreen)
  (|JoinSession (Game|GetPlayerController 0) Session
    (:OnFailure
      (Default|ShowMessageWindow (.AsBP%20Game%20Instance (Utilities|Casting|CastToBP_GameInstance (Game|GetGameInstance))) "Failed to Join Session. Please Try Again.")
      (Viewport|RemoveAllWidgets)
      (CallFunction|ShowMainMenu))))

(event Custom|ShowLoadingScreen
  (Default|ShowLoadingScreen (.AsBP%20Game%20Instance (Utilities|Casting|CastToBP_GameInstance (Game|GetGameInstance)))))

(event Custom|ShowMainMenu
  (bind _returnvalue (Game|GetPlayerController 0))
  (bind _returnvalue_2 (UserInterface|CreateWidget "/Game/MultiplayerGame/Blueprints/Widget/MainMenu/WBP_MainMenu.WBP_MainMenu_C" _returnvalue))
  (UserInterface|Viewport|AddtoViewport _returnvalue_2 0)
  (Variables|/Script/Engine.PlayerController|SetbShowMouseCursor _returnvalue true))

(event Custom|ShowHostMenu
  (bind _returnvalue (UserInterface|CreateWidget "/Game/MultiplayerGame/Blueprints/Widget/MainMenu/WBP_HostMenu.WBP_HostMenu_C" (Game|GetPlayerController 0)))
  (UserInterface|Viewport|AddtoViewport _returnvalue 0))

(fn ConstructionScript)