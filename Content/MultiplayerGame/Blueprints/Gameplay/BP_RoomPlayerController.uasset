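; Player controller for a multiplayer room that manages gameplay UI, chat, scoreboard, game-over screen and pawn input.
; On BeginPlay the local controller creates the overlay and passes player info on, so the game mode respawns the chosen character.
; Chat messages loop through the game mode's connected controllers into each chat box, with H toggling mouse focus.
; Movement, pitch-limited look and fire input are forwarded to the controlled pawn.
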(event Custom|CallServerUpdatePlayerInfo
  (params (PlayerInfo :type F%20Player%20Info%20Structure))
  (Variables|Default|SetPlayerInfo PlayerInfo)
  (bind _asbp_room_game_mode (Utilities|Casting|CastToBP_RoomGameMode (Game|GetGameMode)))
  (Default|RespawnCharacter _asbp_room_game_mode self (.characterclass (Variables|Default|GetPlayerInfo)))
  (CallFunction|CreateGameplayChatBox))

(event Custom|CallPlayerScoreListUpdate
  (bind _gameplayoverlayref (Variables|Default|GetGameplayOverlayRef))
  (Utilities|IsValid _gameplayoverlayref
    (:Is%20Valid
      _)
    (:Is%20Not%20Valid
      (Utilities|FlowControl|Delay 2.0)))
  (Default|RefreshPlayerScoreList _gameplayoverlayref))

(event Custom|UpdateChatMessage
  (params (TextToSend :type Text))
  (Variables|Default|SetSendText TextToSend)
  (Variables|Default|SetSenderName (.name (Variables|Default|GetPlayerInfo)))
  (bind _asbp_room_game_mode (Utilities|Casting|CastToBP_RoomGameMode (Game|GetGameMode)))
  (for _array_element (Variables|/Game/MultiplayerGame/Blueprints/Gameplay/BP_RoomGameMode.BP_RoomGameMode_C|GetConnectedPlayers _asbp_room_game_mode)
    (bind _asbp_room_player_controller (Utilities|Casting|CastToBP_RoomPlayerController _array_element))
    (CallFunction|OnReceiveChatMessage _asbp_room_player_controller (Variables|Default|GetSenderName) (Variables|Default|GetSendText))))

(event Custom|OnReceiveChatMessage
  (params (Sender :type Text) (Message :type Text))
  (Default|UpdateChatLog (Variables|/Game/MultiplayerGame/Blueprints/Widget/Gameplay/WBP_ChatBox_Gameplay.WBP_ChatBox_Gameplay_C|GetGameplayChatBox (Variables|Default|GetGameplayChatBoxRef)) Sender Message))

(event Custom|CreateGameplayChatBox
  (bind _returnvalue (UserInterface|CreateWidget "/Game/MultiplayerGame/Blueprints/Widget/Gameplay/WBP_ChatBox_Gameplay.WBP_ChatBox_Gameplay_C"))
  (bind _output_get (Variables|Default|SetGameplayChatBoxRef _returnvalue))
  (UserInterface|Viewport|AddtoViewport _output_get 0)
  (Variables|Default|SetbShowMouseCursor true))

(event Custom|EndFireOnServer
  (bind _returnvalue (Pawn|GetControlledPawn))
  (Utilities|IsValid _returnvalue
    (:Is%20Valid
      (Class|BPIFire|EndFire(Message) _returnvalue))))

(event Custom|BeginFireOnServer
  (bind _returnvalue (Pawn|GetControlledPawn))
  (Utilities|IsValid _returnvalue
    (:Is%20Valid
      (Class|BPIFire|BeginFire(Message) _returnvalue))))

(event Custom|ShowGameOverOverlay
  (params (WinnerText :type Text))
  (bind _returnvalue (UserInterface|CreateWidget "/Game/MultiplayerGame/Blueprints/Widget/Gameplay/WBP_GameOver.WBP_GameOver_C" 0 WinnerText))
  (UserInterface|Viewport|AddtoViewport _returnvalue 0)
  (Input|SetInputModeUIOnly self _returnvalue "DoNotLock")
  (Variables|Default|SetbShowMouseCursor true))

(event EventBeginPlay
  (if (Pawn|IsLocalController)
    (Viewport|RemoveAllWidgets)
    (CallFunction|CallServerUpdatePlayerInfo (Variables|Default|GetPlayerInfo))
    (bind _returnvalue (UserInterface|CreateWidget "/Game/MultiplayerGame/Blueprints/Widget/Gameplay/WBP_GameplayOverlay.WBP_GameplayOverlay_C"))
    (bind _output_get (Variables|Default|SetGameplayOverlayRef _returnvalue))
    (UserInterface|Viewport|AddtoViewport _output_get 0)
    (else
      (CallFunction|CallPlayerScoreListUpdate))))

(event Input|ActionEvents|InputActionFire
  (params (Key :type Key%20Structure))
  (:Pressed
    (CallFunction|BeginFireonServer))
  (:Released
    (CallFunction|EndFireonServer)))

(event Input|AxisEvents|InputAxisMoveForward
  (params (AxisValue :type Float%20%28single-precision%29))
  (bind _returnvalue (Pawn|GetControlledPawn))
  (Utilities|IsValid _returnvalue
    (:Is%20Valid
      (Pawn|Input|AddMovementInput _returnvalue (Math|Vector|GetForwardVector (Math|Rotator|MakeRotator 0.0 0.0 (.yaw (Pawn|GetControlRotation :!class /Script/Engine.Controller)))) AxisValue false))))

(event Input|AxisEvents|InputAxisMoveRight
  (params (AxisValue :type Float%20%28single-precision%29))
  (bind _returnvalue (Pawn|GetControlledPawn))
  (Utilities|IsValid _returnvalue
    (:Is%20Valid
      (Pawn|Input|AddMovementInput _returnvalue (Math|Vector|GetRightVector (Math|Rotator|MakeRotator 0.0 0.0 (.yaw (Pawn|GetControlRotation :!class /Script/Engine.Controller)))) AxisValue false))))

(event Input|AxisEvents|InputAxisTurn
  (params (AxisValue :type Float%20%28single-precision%29))
  (bind _returnvalue (Pawn|GetControlledPawn))
  (Utilities|IsValid _returnvalue
    (:Is%20Valid
      (Pawn|Input|AddControllerYawInput _returnvalue AxisValue))))

(event Input|AxisEvents|InputAxisLookUp
  (params (AxisValue :type Float%20%28single-precision%29))
  (bind _returnvalue (Pawn|GetControlRotation :!class /Script/Engine.Controller))
  (bind _returnvalue_2 (Pawn|GetControlledPawn))
  (bind _inputpitchscale (Variables|Default|GetInputPitchScale))
  (bind _returnvalue_3 (* AxisValue _inputpitchscale))
  (bind _returnvalue_4 (+ _returnvalue_3 (.pitch _returnvalue)))
  (Utilities|IsValid _returnvalue_2
    (:Is%20Valid
      (if (or (and (> _returnvalue_4 3e+02) (<= _returnvalue_4 999.0)) (and (>= _returnvalue_4 -999.0) (< _returnvalue_4 45.0)))
        (Pawn|Input|AddControllerPitchInput _returnvalue_2 AxisValue)))))

(event Input|KeyboardEvents|H
  (params (Key :type Key%20Structure))
  (bind _self self)
  (:Pressed
    (Utilities|FlowControl|FlipFlop
      (:A
        (Input|SetInputModeGameOnly _self)
        (Variables|Default|SetbShowMouseCursor false))
      (:B
        (Input|SetInputModeGameandUI _self (Variables|Default|GetGameplayChatBoxRef) "DoNotLock" true)
        (Variables|Default|SetbShowMouseCursor true)))))

(fn ConstructionScript)