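; Base gun actor that characters pick up by walking into its sphere trigger.
; Pick runs only if the overlapping BP_BaseCharacter has no valid Weapon, linking both references, disabling mesh physics and attaching the gun to the hand socket.
; Lose clears the gun's owner, re-enables physics and detaches it, but leaves the character's Weapon reference untouched.
; Shoot is an empty function.
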(event OnComponentBeginOverlap(Sphere)
  (params (OverlappedComponent :type Primitive%20Component%20Object%20Reference) (OtherActor :type Actor%20Object%20Reference) (OtherComp :type Primitive%20Component%20Object%20Reference) (OtherBodyIndex :type Integer) (bFromSweep :type Boolean) (SweepResult :type Hit%20Result%20Structure%20%28by%20ref%29))
  (bind _asbp_base_character (Utilities|Casting|CastToBP_BaseCharacter OtherActor))
  (CallFunction|Pick _asbp_base_character))

(event EventBeginPlay)

(event Collision|EventActorBeginOverlap
  (params (OtherActor :type Actor%20Object%20Reference)))

(event EventTick
  (params (DeltaSeconds :type Float%20%28single-precision%29)))

(fn ConstructionScript)

(fn Shoot)

(fn Pick
  (params (持枪者 :type BP%20Base%20Character%20Object%20Reference))
  (Utilities|IsValid (Variables|/Game/MultiplayerGame/Blueprints/Character/BP_BaseCharacter.BP_BaseCharacter_C|GetWeapon 持枪者)
    (:Is%20Not%20Valid
      (bind _output_get (Variables|Default|SetOwnerGun 持枪者))
      (Variables|/Game/MultiplayerGame/Blueprints/Character/BP_BaseCharacter.BP_BaseCharacter_C|SetWeapon _output_get self)
      (Physics|SetSimulatePhysics (Variables|Default|GetSkeletalMesh) false)
      (Transformation|AttachComponentToComponent (Variables|/Script/Engine.Character|GetMesh (Variables|Default|GetOwnerGun)) "hand_rSocket" "SnapToTarget" "SnapToTarget" "KeepRelative" true))))

(fn Lose
  (Variables|Default|SetOwnerGun 0)
  (Physics|SetSimulatePhysics (Variables|Default|GetSkeletalMesh) true)
  (Transformation|DetachFromActor "KeepWorld" "KeepWorld" "KeepRelative"))