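; BP_Gun_3 is a gun variant in the multiplayer game that adds a hitscan-style trace with spark effects to its parent's firing logic.
; Shoot calls the parent, then line traces on the Visibility channel forward from the OwnerGun's FireLocation, with timed debug drawing.
; A sparks emitter spawns at the trace's hit location without checking for a hit, and this override applies no damage itself.
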(event EventBeginPlay
  (|CallParentFunction) ; 此节点被禁用，将不会被调用。\n从引脚连出引线来编译功能。
)

(event Collision|EventActorBeginOverlap
  (params (OtherActor :type Actor%20Object%20Reference))
  (|CallParentFunction OtherActor) ; 此节点被禁用，将不会被调用。\n从引脚连出引线来编译功能。
)

(event EventTick
  (params (DeltaSeconds :type Float%20%28single-precision%29))
  (|CallParentFunction DeltaSeconds) ; 此节点被禁用，将不会被调用。\n从引脚连出引线来编译功能。
)

(fn ConstructionScript
  (|CallParentFunction))

(fn Shoot
  (bind _ownergun (Variables|Default|GetOwnerGun))
  (bind _firelocation (Variables|/Game/MultiplayerGame/Blueprints/Character/BP_BaseCharacter.BP_BaseCharacter_C|GetFireLocation _ownergun))
  (bind _returnvalue (Transformation|GetWorldLocation _firelocation))
  (|CallParentFunction)
  (bind _outhit (Collision|LineTraceByChannel _returnvalue (+ _returnvalue (* (Math|Vector|GetForwardVector _firelocation) 3000)) "TraceTypeQuery1" false 0 "ForDuration"))
  (Effects|SpawnEmitteratLocation "/Game/StarterContent/Particles/P_Sparks.P_Sparks" (.Location (Collision|BreakHitResult _outhit)) "0, 0, 0" "2.000000,2.000000,2.000000"))