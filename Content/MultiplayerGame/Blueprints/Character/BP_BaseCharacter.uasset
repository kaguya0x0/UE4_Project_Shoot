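; Base character for a multiplayer game, handling jump and crouch input and projectile firing.
; Crouch input only sets a flag through an event, while jump calls the built-in character functions.
; BeginFire, with no caller in this graph, spawns a scaled-down BP_Projectile at FireLocation with the character as instigator.
; It then triggers PlayFireEffect, pairing a character fire montage with a weapon animation on a skeletal mesh.
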(event Custom|PlayFireEffect
  (Animation|PlayAnimMontage "/Game/MultiplayerGame/Animations/Fire_Rifle_Hip_Montage.Fire_Rifle_Hip_Montage" 1.0 "Default")
  (Components|Animation|PlayAnimation (Variables|Default|GetSkeletalMesh) "/Game/SciFiWeapDark/Weapons/Anims/Fire_Pistol_W.Fire_Pistol_W" false))

(event Custom|SetCrouchFlag
  (params (CrouchButtonDown :type Boolean))
  (Variables|Default|SetCrouchButtonDown CrouchButtonDown))

(event EventBeginFire
  (bind _firelocation (Variables|Default|GetFireLocation))
  (bind _returnvalue (Transformation|GetWorldTransform _firelocation))
  (Game|SpawnActorfromClass "/Game/MultiplayerGame/Blueprints/Gameplay/BP_Projectile.BP_Projectile_C" (Math|Transform|MakeTransform (.location _returnvalue) (.rotation _returnvalue) "0.500000,0.500000,0.500000") "AdjustIfPossibleButDontSpawnIfColliding" 0 self)
  (CallFunction|PlayFireEffect))

(event Input|ActionEvents|InputActionCrouch
  (params (Key :type Key%20Structure :default "None"))
  (:Pressed
    (CallFunction|SetCrouchFlag true))
  (:Released
    (CallFunction|SetCrouchFlag false)))

(event Input|ActionEvents|InputActionJump
  (params (Key :type Key%20Structure :default "None"))
  (:Pressed
    (if (Character|CanJump)
      (Character|Jump)))
  (:Released
    (Character|StopJumping)))

(fn ConstructionScript)