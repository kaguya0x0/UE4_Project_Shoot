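; BP_AI is a shooter AI in the multiplayer game that fires projectiles and can be killed by players for score.
; A sphere overlap with BP_BaseCharacter toggles the blackboard's CanFire key, while AIFire plays firing animations and spawns BP_Projectile at FireLocation.
; Damage from a room player controller adds score to that player's state, destroys the damage causer and, on the third hit, sets Die before delayed destruction.
; Timer-driven firing logic is left unconnected.
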(event OnComponentBeginOverlap(Sphere)
  (params (OverlappedComponent :type Primitive%20Component%20Object%20Reference) (OtherActor :type Actor%20Object%20Reference) (OtherComp :type Primitive%20Component%20Object%20Reference) (OtherBodyIndex :type Integer) (bFromSweep :type Boolean) (SweepResult :type Hit%20Result%20Structure%20%28by%20ref%29))
  (Utilities|Casting|CastToBP_BaseCharacter OtherActor)
  (AI|Components|Blackboard|SetValueasBool (AI|GetBlackboard (AI|GetAIController self)) (Utilities|Name|MakeLiteralName "CanFire") true))

(event OnComponentEndOverlap(Sphere)
  (params (OverlappedComponent :type Primitive%20Component%20Object%20Reference) (OtherActor :type Actor%20Object%20Reference) (OtherComp :type Primitive%20Component%20Object%20Reference) (OtherBodyIndex :type Integer))
  (Utilities|Casting|CastToBP_BaseCharacter OtherActor)
  (AI|Components|Blackboard|SetValueasBool (AI|GetBlackboard (AI|GetAIController self)) (Utilities|Name|MakeLiteralName "CanFire") false))

(event Custom|AIFire
  (bind _firelocation (Variables|Default|GetFireLocation))
  (bind _returnvalue (Transformation|GetWorldTransform _firelocation))
  (Animation|PlayAnimMontage "/Game/MultiplayerGame/Animations/Fire_Rifle_Hip_Montage.Fire_Rifle_Hip_Montage" 1.0 "Default")
  (Game|SpawnActorfromClass "/Game/MultiplayerGame/Blueprints/Gameplay/BP_Projectile.BP_Projectile_C" (Math|Transform|MakeTransform (.location _returnvalue) (.rotation _returnvalue) (.scale _returnvalue)) "AdjustIfPossibleButDontSpawnIfColliding" 0 self)
  (Components|Animation|PlayAnimation (Variables|Default|GetSkeletalMesh) "/Game/SciFiWeapDark/Weapons/Anims/Fire_Pistol_W.Fire_Pistol_W" false))

(event EventBeginPlay)

(event Game|Damage|EventAnyDamage
  (params (Damage :type Float%20%28single-precision%29) (DamageType :type Damage%20Type%20Object%20Reference) (InstigatedBy :type Controller%20Object%20Reference) (DamageCauser :type Actor%20Object%20Reference))
  (bind _asbp_room_player_controller (Utilities|Casting|CastToBP_RoomPlayerController InstigatedBy))
  (bind _asbp_room_player_state (Utilities|Casting|CastToBP_RoomPlayerState (Variables|/Script/Engine.Controller|GetPlayerState _asbp_room_player_controller)))
  (Default|UpdateScore _asbp_room_player_state 1.0)
  (Actor|DestroyActor DamageCauser)
  (Variables|Default|SetHurtNum (+ (Variables|Default|GetHurtNum) 1))
  (if (> (Math|Conversions|ToByte(Integer) (Variables|Default|GetHurtNum)) 2)
    (Variables|Default|SetDie true)
    (Utilities|FlowControl|Delay 2.0)
    (Actor|DestroyActor)))

(fn ConstructionScript)