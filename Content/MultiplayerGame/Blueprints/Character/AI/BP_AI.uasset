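; BP_AI is an AI character Blueprint in the multiplayer game, currently an unfinished stub with no active behavior.
; A custom event moves the pawn to a random navigable point within a radius of itself, but its initial call and randomized looping timer are disconnected.
; Sphere overlap events cast the overlapped component, rather than the other actor, to BP_BaseCharacter and do nothing further.
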(event OnComponentBeginOverlap(Sphere)
  (params (OverlappedComponent :type Primitive%20Component%20Object%20Reference) (OtherActor :type Actor%20Object%20Reference) (OtherComp :type Primitive%20Component%20Object%20Reference) (OtherBodyIndex :type Integer) (bFromSweep :type Boolean) (SweepResult :type Hit%20Result%20Structure%20%28by%20ref%29))
  (Utilities|Casting|CastToBP_BaseCharacter OverlappedComponent))

(event OnComponentEndOverlap(Sphere)
  (params (OverlappedComponent :type Primitive%20Component%20Object%20Reference) (OtherActor :type Actor%20Object%20Reference) (OtherComp :type Primitive%20Component%20Object%20Reference) (OtherBodyIndex :type Integer))
  (Utilities|Casting|CastToBP_BaseCharacter OverlappedComponent))

(event Custom|AI移动
  (AI|AIMoveTo self (.RandomLocation (Class|NavigationSystemV1|GetRandomPointinNavigableRadius (Transformation|GetActorLocation) 5e+03 0 0)) 0 5.0 false))

(event EventBeginPlay)

(fn ConstructionScript)