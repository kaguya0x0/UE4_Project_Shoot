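; Magic AI enemy that attacks BP_Pineapple and awards score to players who damage it.
; Sphere overlap with the pineapple starts a looping attack animation and sets CanAttack, also mirrored to the Blackboard; Tick then drains the GameState NPC's HP about once per second.
; End overlap with a BP_BaseCharacter clears only the Blackboard flag.
; Player hits destroy the damage causer; the third plays a death animation, then destroys the enemy after a delay.
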(event OnComponentBeginOverlap(Sphere)
  (params (OverlappedComponent :type Primitive%20Component%20Object%20Reference) (OtherActor :type Actor%20Object%20Reference) (OtherComp :type Primitive%20Component%20Object%20Reference) (OtherBodyIndex :type Integer) (bFromSweep :type Boolean) (SweepResult :type Hit%20Result%20Structure%20%28by%20ref%29))
  (Utilities|Casting|CastToBP_Pineapple OtherActor)
  (Variables|Default|SetCanAttack true)
  (AI|Components|Blackboard|SetValueasBool (AI|GetBlackboard (AI|GetAIController self)) (Utilities|Name|MakeLiteralName "CanAttack") true)
  (Components|Animation|PlayAnimation (Variables|Character|GetMesh) "/Game/BattleWizardPolyart/Animations/Attack01Anim.Attack01Anim" true))

(event OnComponentEndOverlap(Sphere)
  (params (OverlappedComponent :type Primitive%20Component%20Object%20Reference) (OtherActor :type Actor%20Object%20Reference) (OtherComp :type Primitive%20Component%20Object%20Reference) (OtherBodyIndex :type Integer))
  (Utilities|Casting|CastToBP_BaseCharacter OtherActor)
  (AI|Components|Blackboard|SetValueasBool (AI|GetBlackboard (AI|GetAIController self)) (Utilities|Name|MakeLiteralName "CanAttack") false))

(event EventBeginPlay
  (Rendering|Material|SetMaterial (Variables|Character|GetMesh) 0 (Utilities|Select :Index (Math|Random|RandomIntegerinRange 0 3) :Option%200 "/Game/BattleWizardPolyart/Materials/MaskTintPolyartMat.MaskTintPolyartMat" :Option%201 "/Game/BattleWizardPolyart/Materials/MaskTintPolyartMatInst01.MaskTintPolyartMatInst01" :Option%202 "/Game/BattleWizardPolyart/Materials/MaskTintPolyartMatInst02.MaskTintPolyartMatInst02")))

(event EventTick
  (params (DeltaSeconds :type Float%20%28single-precision%29))
  (bind _returnvalue (Game|GetGameState))
  (bind _asbp_room_game_state (Utilities|Casting|CastToBP_RoomGameState _returnvalue))
  (bind _npc (Variables|/Game/MultiplayerGame/Blueprints/Gameplay/BP_RoomGameState.BP_RoomGameState_C|GetNPC _asbp_room_game_state))
  (if (Variables|Default|GetCanAttack)
    (Variables|Default|Settimer (+ DeltaSeconds (Variables|Default|Gettimer)))
    (if (> (Variables|Default|Gettimer) 1.0)
      (Default|NPCHurt _asbp_room_game_state)
      (Variables|/Game/MultiplayerGame/Blueprints/Character/NPC/BP_Pineapple.BP_Pineapple_C|SetHP _npc (- (Variables|/Game/MultiplayerGame/Blueprints/Character/NPC/BP_Pineapple.BP_Pineapple_C|GetHP _npc) 1))
      (Variables|Default|Settimer 0.0))))

(event Game|Damage|EventAnyDamage
  (params (Damage :type Float%20%28single-precision%29) (DamageType :type Damage%20Type%20Object%20Reference) (InstigatedBy :type Controller%20Object%20Reference) (DamageCauser :type Actor%20Object%20Reference))
  (bind _as玩家控制器 (Utilities|Casting|CastToPlayerController InstigatedBy))
  (bind _asbp_room_player_state (Utilities|Casting|CastToBP_RoomPlayerState (Variables|/Script/Engine.Controller|GetPlayerState _as玩家控制器)))
  (Default|UpdateScore _asbp_room_player_state 1.0)
  (Actor|DestroyActor DamageCauser)
  (Variables|Default|SetHurtNum (+ (Variables|Default|GetHurtNum) 1))
  (if (> (Math|Conversions|ToByte(Integer) (Variables|Default|GetHurtNum)) 2)
    (Variables|Default|SetDie true)
    (Components|Animation|PlayAnimation (Variables|Character|GetMesh) "/Game/BattleWizardPolyart/Animations/DieAnim.DieAnim" false)
    (Utilities|FlowControl|Delay 3.0)
    (Actor|DestroyActor)))

(fn ConstructionScript)