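; BP_Pineapple is an NPC in the multiplayer game that tracks hits and reports them to the room game state.
; On BeginPlay it registers itself as the NPC on BP_RoomGameState.
; Any damage event, whatever its amount, takes one point off HP, prints the new value and calls NPCHurt on the game state.
; It has no death or zero-HP handling of its own.
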(event EventBeginPlay
  (bind _asbp_room_game_state (Utilities|Casting|CastToBP_RoomGameState (Game|GetGameState)))
  (Variables|/Game/MultiplayerGame/Blueprints/Gameplay/BP_RoomGameState.BP_RoomGameState_C|SetNPC _asbp_room_game_state self))

(event Collision|EventActorBeginOverlap
  (params (OtherActor :type Actor%20Object%20Reference)))

(event EventTick
  (params (DeltaSeconds :type Float%20%28single-precision%29)))

(event Game|Damage|EventAnyDamage
  (params (Damage :type Float%20%28single-precision%29) (DamageType :type Damage%20Type%20Object%20Reference) (InstigatedBy :type Controller%20Object%20Reference) (DamageCauser :type Actor%20Object%20Reference))
  (Variables|Default|SetHP (- (Variables|Default|GetHP) 1))
  (Development|PrintString (Utilities|String|ToString(Integer) (Variables|Default|GetHP)))
  (bind _asbp_room_game_state (Utilities|Casting|CastToBP_RoomGameState (Game|GetGameState)))
  (Default|NPCHurt _asbp_room_game_state))

(fn ConstructionScript)