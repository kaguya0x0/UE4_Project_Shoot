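; Lobby player controller for a multiplayer game, owning the lobby menu and handling kicks, loading screen and pawn movement, clamped look and fire input.
; It loads or generates the saved profile, then passes player info to BP_LobbyGameMode to swap characters and update clients.
; Character selection reserves slots in the game mode's availability array, except always-selectable index 0.
; Chat fans out through connected controllers, and H toggles menu panels and input mode.
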(event Custom|Kicked
  (params (KickReason :type Text))
  (bind _returnvalue (Game|GetGameInstance))
  (bind _asbp_game_instance (Utilities|Casting|CastToBP_GameInstance _returnvalue))
  (Utilities|FlowControl|Sequence
    (:then_0
      (Default|LeaveGame _asbp_game_instance self))
    (:then_1
      (Default|ShowMessageWindow _asbp_game_instance KickReason))
    (:then_2
      (Game|OpenLevel(byName) "MainMenu"))))

(event Custom|InitialPlayerInfo
  (CallFunction|UpdateSavedProfile)
  (CallFunction|CallServerUpdatePlayerInfo (Variables|Default|GetPlayerInfo) true))

(event Custom|UpdateCharacterInfo
  (params (CharacterClass :type BP%20Base%20Character%20Class%20Reference) (CharacterImage :type Texture%202D%20Object%20Reference))
  (bind _structout (Utilities|Struct|SetmembersinFPlayerInfo (Variables|Default|GetPlayerInfo) CharacterClass CharacterImage))
  (bind _returnvalue (SaveGame|CreateSaveGameObject "/Game/MultiplayerGame/Blueprints/General/BP_SavedPlayerProfile.BP_SavedPlayerProfile_C"))
  (Default|SaveProfile (.AsBP%20Game%20Instance (Utilities|Casting|CastToBP_GameInstance (Game|GetGameInstance))) _returnvalue _structout)
  (CallFunction|CallServerUpdatePlayerInfo (Variables|Default|GetPlayerInfo) true))

(event Custom|UpdateChatMessage
  (params (TextToSend :type Text))
  (Variables|Default|SetSendText TextToSend)
  (Variables|Default|SetSenderName (.name (Variables|Default|GetPlayerInfo)))
  (bind _asbp_lobby_game_mode (Utilities|Casting|CastToBP_LobbyGameMode (Game|GetGameMode)))
  (for _array_element (Variables|/Game/MultiplayerGame/Blueprints/Lobby/BP_LobbyGameMode.BP_LobbyGameMode_C|GetConnectedPlayers _asbp_lobby_game_mode)
    (bind _asbp_lobby_player_controller (Utilities|Casting|CastToBP_LobbyPlayerController _array_element))
    (CallFunction|OnReceiveChatMessage _asbp_lobby_player_controller (Variables|Default|GetSenderName) (Variables|Default|GetSendText))))

(event Custom|OnReceiveChatMessage
  (params (Sender :type Text) (Message :type Text))
  (Default|UpdateChatLog (Variables|/Game/MultiplayerGame/Blueprints/Widget/Lobby/WBP_LobbyMenu.WBP_LobbyMenu_C|GetChatBoxWindow (Variables|Default|GetLobbyMenuRef)) Sender Message))

(event Custom|SelectCharacter
  (params (CharacterIndex :type Integer) (CharacterImage :type Texture%202D%20Object%20Reference))
  (bind _returnvalue (Game|GetGameMode))
  (bind _asbp_lobby_game_mode (Utilities|Casting|CastToBP_LobbyGameMode _returnvalue))
  (bind _availablecharacters (Variables|/Game/MultiplayerGame/Blueprints/Lobby/BP_LobbyGameMode.BP_LobbyGameMode_C|GetAvailableCharacters _asbp_lobby_game_mode))
  (Variables|Default|SetPreviousSelectCharacterIndex (Variables|Default|GetCurrentSelectCharacterIndex))
  (Variables|Default|SetCurrentSelectCharacterIndex CharacterIndex)
  (Variables|Default|SetCurrentSelectCharacterImage CharacterImage)
  (if (== 0 (Variables|Default|GetCurrentSelectCharacterIndex))
    (Utilities|Array|SetArrayElem _availablecharacters (Variables|Default|GetPreviousSelectCharacterIndex) true :!label _label)
    (CallFunction|UpdateCharacterInfo (Utilities|Array|Get(acopy) (Variables|/Game/MultiplayerGame/Blueprints/Lobby/BP_LobbyGameMode.BP_LobbyGameMode_C|GetCharactersClass _asbp_lobby_game_mode) (Variables|Default|GetCurrentSelectCharacterIndex)) (Variables|Default|GetCurrentSelectCharacterImage))
    (elif (not (Math|Boolean|Equal(Boolean) (Utilities|Array|Get(acopy) _availablecharacters (Variables|Default|GetCurrentSelectCharacterIndex)) false))
      (Utilities|Array|SetArrayElem _availablecharacters (Variables|Default|GetCurrentSelectCharacterIndex) false)
      (goto _label))))

(event Custom|CreateLobbyMenu
  (params (ServerName :type Text))
  (Variables|Default|SetbShowMouseCursor true)
  (bind _returnvalue (UserInterface|CreateWidget "/Game/MultiplayerGame/Blueprints/Widget/Lobby/WBP_LobbyMenu.WBP_LobbyMenu_C" self (Utilities|Text|ToText(String) (Utilities|String|Append "Server Name: " (Utilities|String|ToString(Text) ServerName)))))
  (bind _output_get (Variables|Default|SetLobbyMenuRef _returnvalue))
  (UserInterface|Viewport|AddtoViewport _output_get 0)
  (Input|SetInputModeGameandUI self _output_get "DoNotLock" true))

(event Custom|CallServerUpdatePlayerInfo
  (params (PlayerInfo :type F%20Player%20Info%20Structure) (NeedSwapCharacter :type Boolean))
  (bind _output_get (Variables|Default|SetPlayerInfo PlayerInfo))
  (bind _asbp_lobby_game_mode (Utilities|Casting|CastToBP_LobbyGameMode (Game|GetGameMode)))
  (if NeedSwapCharacter
    (Default|SwapCharacter _asbp_lobby_game_mode self (.characterclass _output_get)))
  (Default|UpdateClients _asbp_lobby_game_mode))

(event Custom|EndFireOnServer
  (bind _returnvalue (Pawn|GetControlledPawn))
  (Utilities|IsValid _returnvalue
    (:Is%20Valid
      (Class|BPIFire|EndFire(Message) _returnvalue))))

(event Custom|BeginFireOnServer
  (bind _returnvalue (Pawn|GetControlledPawn))
  (Utilities|IsValid _returnvalue
    (:Is%20Valid
      (Class|BPIFire|BeginFire(Message) _returnvalue))))

(event Custom|UpdateLobbySettings
  (params (MapImage :type Texture%202D%20Object%20Reference) (MapName :type Text) (MapTime :type Text))
  (bind _lobbymenuref (Variables|Default|GetLobbyMenuRef))
  (Utilities|IsValid _lobbymenuref
    (:Is%20Valid
      (Variables|/Game/MultiplayerGame/Blueprints/Widget/Lobby/WBP_LobbyMenu.WBP_LobbyMenu_C|SetMapTexture _lobbymenuref MapImage)
      (Variables|/Game/MultiplayerGame/Blueprints/Widget/Lobby/WBP_LobbyMenu.WBP_LobbyMenu_C|SetMapName _lobbymenuref MapName)
      (Variables|/Game/MultiplayerGame/Blueprints/Widget/Lobby/WBP_LobbyMenu.WBP_LobbyMenu_C|SetMapTime _lobbymenuref MapTime))))

(event Custom|UpdatePlayerNumDisplayText
  (params (CurrentPlayer :type Integer) (MaxPlayer :type Integer))
  (bind _lobbymenuref (Variables|Default|GetLobbyMenuRef))
  (Utilities|IsValid _lobbymenuref
    (:Is%20Valid
      (Variables|/Game/MultiplayerGame/Blueprints/Widget/Lobby/WBP_LobbyMenu.WBP_LobbyMenu_C|SetPlayerNumDisplayText _lobbymenuref (Utilities|Text|ToText(String) (Utilities|String|Append (Utilities|String|ToString(Integer) CurrentPlayer) " of " (Utilities|String|ToString(Integer) MaxPlayer)))))))

(event Custom|UpdatePlayerInfoList
  (params (ConnectedPlayersInfo :type Array%20of%20F%20Player%20Info%20Structures))
  (bind _lobbymenuref (Variables|Default|GetLobbyMenuRef))
  (Utilities|IsValid _lobbymenuref
    (:Is%20Valid
      (Default|ClearPlayerInfoList _lobbymenuref)
      (for _array_element ConnectedPlayersInfo
        (Default|AddConnectedPlayerInfo _lobbymenuref _array_element)))))

(event Custom|UpdateAvailableCharacters
  (params (AvailableCharacters :type Array%20of%20Booleans))
  (bind _lobbymenuref (Variables|Default|GetLobbyMenuRef))
  (Utilities|IsValid _lobbymenuref
    (:Is%20Valid
      (for (_array_element _array_index) (Variables|/Game/MultiplayerGame/Blueprints/Widget/Lobby/WBP_CharacterSelectWindow.WBP_CharacterSelectWindow_C|GetCharacterSelectButtons (Variables|/Game/MultiplayerGame/Blueprints/Widget/Lobby/WBP_LobbyMenu.WBP_LobbyMenu_C|GetSelectCharacterWindow _lobbymenuref))
        (Widget|SetIsEnabled _array_element (Utilities|Array|Get(acopy) AvailableCharacters _array_index))))))

(event Custom|ShowLoadingScreen
  (Widget|RemovefromParent (Variables|Default|GetLobbyMenuRef))
  (Default|ShowLoadingScreen (.AsBP%20Game%20Instance (Utilities|Casting|CastToBP_GameInstance (Game|GetGameInstance)))))

(event Input|ActionEvents|InputActionFire
  (params (Key :type Key%20Structure :default "None"))
  (:Pressed
    (CallFunction|BeginFireonServer))
  (:Released
    (CallFunction|EndFireonServer)))

(event Input|AxisEvents|InputAxisMoveForward
  (params (AxisValue :type Float%20%28single-precision%29))
  (bind _returnvalue (Pawn|GetControlledPawn))
  (Utilities|IsValid _returnvalue
    (:Is%20Valid
      (Pawn|Input|AddMovementInput _returnvalue (Math|Vector|GetForwardVector (Math|Rotator|MakeRotator 0.0 0.0 (.yaw (Pawn|GetControlRotation :!class /Script/Engine.Controller)))) AxisValue false))))

(event Input|AxisEvents|InputAxisMoveRight
  (params (AxisValue :type Float%20%28single-precision%29))
  (bind _returnvalue (Pawn|GetControlledPawn))
  (Utilities|IsValid _returnvalue
    (:Is%20Valid
      (Pawn|Input|AddMovementInput _returnvalue (Math|Vector|GetRightVector (Math|Rotator|MakeRotator 0.0 0.0 (.yaw (Pawn|GetControlRotation :!class /Script/Engine.Controller)))) AxisValue false))))

(event Input|AxisEvents|InputAxisTurn
  (params (AxisValue :type Float%20%28single-precision%29))
  (bind _returnvalue (Pawn|GetControlledPawn))
  (Utilities|IsValid _returnvalue
    (:Is%20Valid
      (Pawn|Input|AddControllerYawInput _returnvalue AxisValue))))

(event Input|AxisEvents|InputAxisLookUp
  (params (AxisValue :type Float%20%28single-precision%29))
  (bind _returnvalue (Pawn|GetControlRotation :!class /Script/Engine.Controller))
  (bind _returnvalue_2 (Pawn|GetControlledPawn))
  (bind _inputpitchscale (Variables|Default|GetInputPitchScale))
  (bind _returnvalue_3 (* AxisValue _inputpitchscale))
  (bind _returnvalue_4 (+ _returnvalue_3 (.pitch _returnvalue)))
  (Utilities|IsValid _returnvalue_2
    (:Is%20Valid
      (if (or (and (> _returnvalue_4 3e+02) (<= _returnvalue_4 999.0)) (and (>= _returnvalue_4 -999.0) (< _returnvalue_4 45.0)))
        (Pawn|Input|AddControllerPitchInput _returnvalue_2 AxisValue)))))

(event Input|KeyboardEvents|H
  (params (Key :type Key%20Structure :default "None"))
  (bind _self self)
  (bind _lobbymenuref (Variables|Default|GetLobbyMenuRef))
  (bind _lobbysettingswindow (Variables|/Game/MultiplayerGame/Blueprints/Widget/Lobby/WBP_LobbyMenu.WBP_LobbyMenu_C|GetLobbySettingsWindow _lobbymenuref))
  (:Pressed
    (Utilities|FlowControl|FlipFlop
      (:A
        (Widget|SetVisibility _lobbysettingswindow "Hidden")
        (Input|SetInputModeGameOnly _self)
        (Variables|Default|SetbShowMouseCursor false))
      (:B
        (Widget|SetVisibility _lobbysettingswindow "Visible")
        (Input|SetInputModeGameandUI _self _lobbymenuref "DoNotLock" true)
        (Variables|Default|SetbShowMouseCursor true)))))

(fn ConstructionScript)

(fn UpdateSavedProfile
  (bind _returnvalue (Game|GetGameInstance))
  (bind _asbp_game_instance (Utilities|Casting|CastToBP_GameInstance _returnvalue))
  (bind _doessavegameexist (Default|CheckSavedProfile _asbp_game_instance))
  (if _doessavegameexist
    (bind _savedplayerinfo (Default|LoadProfile _asbp_game_instance))
    (bind _returnvalue_2 (SaveGame|CreateSaveGameObject "/Game/MultiplayerGame/Blueprints/General/BP_SavedPlayerProfile.BP_SavedPlayerProfile_C"))
    (Utilities|Struct|SetmembersinFPlayerInfo (Variables|Default|GetPlayerInfo) (.Name (Utilities|Struct|BreakFPlayerInfo _savedplayerinfo)) (.Avatar (Utilities|Struct|BreakFPlayerInfo _savedplayerinfo)))
    (Default|SaveProfile _asbp_game_instance _returnvalue_2 (Variables|Default|GetPlayerInfo))
    (else
      (bind _returnvalue_3 (SaveGame|CreateSaveGameObject "/Game/MultiplayerGame/Blueprints/General/BP_SavedPlayerProfile.BP_SavedPlayerProfile_C"))
      (Utilities|Struct|SetmembersinFPlayerInfo (Variables|Default|GetPlayerInfo) (Utilities|Text|ToText(String) (Utilities|String|Append "Player_" (.LeftS (Utilities|String|Split (Guid|ToString(Guid) (Guid|NewGuid)) "-")))))
      (Default|SaveProfile _asbp_game_instance _returnvalue_3 (Variables|Default|GetPlayerInfo)))))